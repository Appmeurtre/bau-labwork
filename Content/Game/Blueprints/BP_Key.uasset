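; BP_Key is an interactable key pickup that records its key number in the game mode when claimed.
; On BeginPlay it caches BP_Gamemode, and Interact overwrites that game mode's Keys value with its KeyNumber.
; It then prints a claimed message using the matching entry in Names and destroys itself.
; The construction script applies the Material variable to the Key component, so each instance can look different.
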(event `self.ReceiveBeginPlay`
  (bind _asbp_gamemode (cast `/Game/Game/Core/BP_Gamemode` (`GameplayStatics.GetGameMode`)))
  (set `self.BP_Gamemode` _asbp_gamemode))

(event `/Game/Game/Blueprints/BPI_Interact.Interact`
  (bind _output_get (set `/Game/Game/Core/BP_Gamemode.Keys` (`self.KeyNumber`) (`self.BP_Gamemode`)))
  (`KismetSystemLibrary.PrintString` (`KismetStringLibrary.Concat_StrStr` "Key" (`|GetArrayItem` (`self.Names`) _output_get) "Claimed!") true true (struct :`R` 1.0 :`G` 0.943689 :`A` 1.0))
  (`self.K2_DestroyActor`))

(fn `UserConstructionScript`
  (`PrimitiveComponent.SetMaterial` (`self.Key`) 0 (`self.Material`)))