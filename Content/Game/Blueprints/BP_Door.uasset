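; BP_Door is a locked door Blueprint that opens on Interact when the game mode's key value matches its key number.
; It caches BP_Gamemode on BeginPlay and compares its Keys to KeyNumber exactly, printing an error on a mismatch.
; On a match, the Door_Rotate timeline slides the mesh between start and finish locations, despite its name.
; The construction script applies the door's material and a fixed scale.
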(event `self.ReceiveBeginPlay`
  (bind _asbp_gamemode (cast `/Game/Game/Core/BP_Gamemode` (`GameplayStatics.GetGameMode`)))
  (set `self.BP_Gamemode` _asbp_gamemode))

(event `/Game/Game/Blueprints/BPI_Interact.Interact`
  (if (== (`/Game/Game/Core/BP_Gamemode.Keys` (`self.BP_Gamemode`)) (`self.KeyNumber`))
    (bind (_direction _newtrack_0) (`Timeline|Door_Rotate`)
      (:`Update`
        (`SceneComponent.K2_SetRelativeLocation` (`self.SM_Door`) (`KismetMathLibrary.VLerp` (`self.StartLocation`) (`self.FinishLocation`) _newtrack_0) false false)))
    (else
      (`KismetSystemLibrary.PrintString` "INCORRECT KEY" true true (struct :`R` 0.390301 :`B` 1.0 :`A` 1.0)))))

(fn `UserConstructionScript`
  (`PrimitiveComponent.SetMaterial` (`self.SM_Door`) 0 (`self.Material`))
  (`SceneComponent.SetRelativeScale3D` (`self.SM_Door`) (5.0 5.0 0.5)))